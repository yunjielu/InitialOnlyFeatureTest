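; PlayerCharacter_BP is a player character Blueprint that shows a live debug readout of its own and its components' variables.
; Each Tick, it sets the TextRender color and rebuilds its text from labeled values, one per line.
; The values come from parent and actor variables, parent and own variables of the first MyActorComponent entry, and a SubActorComponent variable.
; BeginPlay, overlap and the construction script are empty.
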(event EventBeginPlay)

(event Collision|EventActorBeginOverlap
  (params (OtherActor :type Actor%20Object%20Reference)))

(event EventTick
  (params (DeltaSeconds :type Float%20%28single-precision%29))
  (bind _myactorcomponent (Variables|Default|GetMyActorComponent))
  (bind _textrender (Variables|Default|GetTextRender))
  (bind _output (Utilities|Array|Get(acopy) _myactorcomponent))
  (Rendering|Components|TextRender|SetTextRenderColor _textrender (Math|Color|MakeColor 0 0 191))
  (Rendering|Components|TextRender|SetText _textrender (Utilities|Text|ToText(String) (Utilities|String|Append "ActorParent:" (Utilities|String|ToString(Integer) (Variables|Default|GetActorParentVar2)) "<br>Actor:" (Utilities|String|ToString(Integer) (Variables|Default|GetActorVar2)) "<br>MyCompParent:" (Utilities|String|ToString(Integer) (Variables|/Script/InitialOnlyFeature.MyActorComponentParent|GetMyComponentParentVar2 _output)) "<br>MyComp:" (Utilities|String|ToString(Integer) (Variables|/Script/InitialOnlyFeature.MyActorComponent|GetMyComponentVar2 _output)) "<br>SubComp:" (Utilities|String|ToString(Integer) (Variables|/Script/InitialOnlyFeature.SubActorComponent|GetSubComponentVar2 (Variables|Default|GetSubActorComponent)))))))

(fn ConstructionScript)